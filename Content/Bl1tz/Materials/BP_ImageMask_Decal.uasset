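; BP_ImageMask_Decal is a configurable decal actor that projects a chosen texture and normal map.
; Its construction script creates a dynamic instance of DecalMaterial and feeds it the actor's variables for textures, color, hue, normal intensity, stretch, offset and tiling.
; It then assigns that instance and a sort order to the Decal component.
; All work happens at construction, with no active runtime events.
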(event EventBeginPlay)

(event Collision|EventActorBeginOverlap
  (params (OtherActor :type Actor%20Object%20Reference)))

(event EventTick
  (params (DeltaSeconds :type Float%20%28single-precision%29)))

(fn ConstructionScript
  (bind _decal (Variables|Default|GetDecal))
  (bind _returnvalue (Rendering|Material|CreateDynamicMaterialInstance (Variables|Default|GetDecal%20Material) "None" "None" :!class /Script/Engine.KismetMaterialLibrary))
  (bind _output_get (Variables|Default|SetDecal%20Instance _returnvalue))
  (Rendering|Material|SetTextureParameterValue (Variables|Default|GetDecal%20Instance) "Diffuse" (Variables|Decal|GetDecal%20Texture))
  (Rendering|Material|SetTextureParameterValue (Variables|Default|GetDecal%20Instance) "Normal" (Variables|Decal|GetDecal%20Texture%20Normal))
  (Rendering|Material|SetVectorParameterValue (Variables|Default|GetDecal%20Instance) "Color" (Math|Conversions|ToLinearColor(Float) (Variables|Decal|GetColor%20Str)) :!class /Script/Engine.MaterialInstanceDynamic)
  (Rendering|Material|SetScalarParameterValue (Variables|Default|GetDecal%20Instance) "Normal Intensity" (Variables|Decal|GetNormal%20Str) :!class /Script/Engine.MaterialInstanceDynamic)
  (Rendering|Material|SetScalarParameterValue (Variables|Default|GetDecal%20Instance) "Hue" (Variables|Decal|GetHue) :!class /Script/Engine.MaterialInstanceDynamic)
  (Rendering|Material|SetScalarParameterValue (Variables|Default|GetDecal%20Instance) "Stretch X (S)" (Variables|UVs|GetStretch%20X) :!class /Script/Engine.MaterialInstanceDynamic)
  (Rendering|Material|SetScalarParameterValue (Variables|Default|GetDecal%20Instance) "Stretch Y (S)" (Variables|UVs|GetStretch%20Y) :!class /Script/Engine.MaterialInstanceDynamic)
  (Rendering|Material|SetScalarParameterValue (Variables|Default|GetDecal%20Instance) "Move X (S)" (Variables|UVs|GetMove%20X) :!class /Script/Engine.MaterialInstanceDynamic)
  (Rendering|Material|SetScalarParameterValue (Variables|Default|GetDecal%20Instance) "Move Y (S)" (Variables|UVs|GetMove%20Y) :!class /Script/Engine.MaterialInstanceDynamic)
  (Rendering|Material|SetScalarParameterValue (Variables|Default|GetDecal%20Instance) "Density (S)" (Variables|UVs|GetUV%20Tile) :!class /Script/Engine.MaterialInstanceDynamic)
  (Rendering|Components|Decal|SetDecalMaterial _decal (Variables|Default|GetDecal%20Instance))
  (Class|DecalComponent|SetSortOrder _decal (Variables|Decal|GetSort%20Order)))