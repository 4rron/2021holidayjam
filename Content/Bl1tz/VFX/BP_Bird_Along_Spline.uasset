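; Bird VFX actor that moves a Niagara bird and a dummy bird along a spline.
; On BeginPlay the SplineAnim timeline's play rate becomes the inverse of NewTime, and its alpha is scaled by spline length into a distance.
; Each update sets both birds' local location and aims them along the tangent, offset by a Rotation variable.
; The construction script toggles dummy bird visibility through ShowDummyBird.
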(event EventBeginPlay
  (bind _spline (Variables|Default|GetSpline))
  (bind _spline_anim (Variables|Default|GetSpline%20Anim))
  (bind _returnvalue (Components|Timeline|GetTimelineLength _spline_anim))
  (Components|Timeline|SetPlayRate _spline_anim (/ _returnvalue (* _returnvalue (Variables|Default|GetNew%20Time))))
  (bind _0_1 (Timeline|Spline%20Anim SetNewTime)
    (:Update
      (Transformation|SetRelativeLocationAndRotation (Variables|Default|GetDummy%20Bird) (Spline|GetLocationatDistanceAlongSpline _spline (* _0_1 (Spline|GetSplineLength _spline)) "Local") (Math|Conversions|RotationFromXVector (Math|Vector|RotateVector (Spline|GetTangentatDistanceAlongSpline _spline (* _0_1 (Spline|GetSplineLength _spline)) "Local") (Variables|Default|GetRotation))) false false))))

(fn ConstructionScript
  (Rendering|SetVisibility (Variables|Default|GetDummy%20Bird) (Variables|Default|GetShow%20Dummy%20Bird%20?) false))